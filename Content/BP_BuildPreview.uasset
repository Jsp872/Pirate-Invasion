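; BP_BuildPreview is a building placement preview that shows the chosen building's mesh and tracks what overlaps its footprint.
; SetBuildingClass copies the mesh from the building class defaults onto its StaticMesh.
; Box overlap events keep a unique list of player builder units inside the area and count every other overlapping actor as a blocker.
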(event `SetBuildingClass`
  (params (BuildingClass :type "/Game/BP_Building Class Reference"))
  (`StaticMeshComponent.SetStaticMesh` (`self.StaticMesh`) (defaults `Object` BuildingClass)))

(event `self.Box.OnComponentBeginOverlap`
  (params (OverlappedComponent :type "PrimitiveComponent Object Reference") (OtherActor :type "Actor Object Reference") (OtherComp :type "PrimitiveComponent Object Reference") (OtherBodyIndex :type Integer) (bFromSweep :type Boolean) (SweepResult :type "HitResult Structure (by ref)"))
  (bind _asbp_strategy_unit_player_builder (cast `/Game/Variant_Strategy/Blueprints/BP_StrategyUnitPlayerBuilder` OtherActor)
    (:`then`
      (`KismetArrayLibrary.Array_AddUnique` (`self.ListOfConstructor`) _asbp_strategy_unit_player_builder))
    (:`CastFailed`
      (`/Engine/EditorBlueprintResources/StandardMacros.IncrementInt` (`self.BlockingActors`)))))

(event `self.Box.OnComponentEndOverlap`
  (params (OverlappedComponent :type "PrimitiveComponent Object Reference") (OtherActor :type "Actor Object Reference") (OtherComp :type "PrimitiveComponent Object Reference") (OtherBodyIndex :type Integer))
  (bind _asbp_strategy_unit_player_builder (cast `/Game/Variant_Strategy/Blueprints/BP_StrategyUnitPlayerBuilder` OtherActor)
    (:`then`
      (`KismetArrayLibrary.Array_RemoveItem` (`self.ListOfConstructor`) _asbp_strategy_unit_player_builder))
    (:`CastFailed`
      (`/Engine/EditorBlueprintResources/StandardMacros.DecrementInt` (`self.BlockingActors`)))))

(fn `UserConstructionScript`)
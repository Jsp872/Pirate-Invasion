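; BP_Ressources is a resource node that holds a randomized amount and can respawn after being used up.
; On BeginPlay it rolls Amount between a min and max and caches the cube's material and the per-collection give value.
; RestoreRessource zeroes that give value and turns the cube red, waits a respawn delay, then rerolls Amount and restores both the material and give value.
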(event `self.ReceiveBeginPlay`
  (set `self.Amount` (`KismetMathLibrary.RandomIntegerInRange` (`self.MinAmount`) (`self.MaxAmount`)))
  (set `self.MaterialSave` (`PrimitiveComponent.GetMaterial` (`self.Cube`) 0))
  (set `self.SaveAmountToGive` (`self.AmountToGive`)))

(event `Restore Ressource`
  (set `self.AmountToGive` 0)
  (`PrimitiveComponent.SetMaterial` (`self.Cube`) 0 "/Game/M_Red.M_Red")
  (`KismetSystemLibrary.Delay` (`self.WaitingTimeForRespawnOffRessource`))
  (set `self.Amount` (`KismetMathLibrary.RandomIntegerInRange` (`self.MinAmount`) (`self.MaxAmount`)))
  (`PrimitiveComponent.SetMaterial` (`self.Cube`) 0 (`self.MaterialSave`))
  (set `self.AmountToGive` (`self.SaveAmountToGive`)))

(fn `UserConstructionScript`)
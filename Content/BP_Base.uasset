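; BP_Base is a base actor that registers itself with the game state as its Base.
; On BeginPlay it calls the parent event, casts the game state to BP_GameState and stores a self reference in its Base variable.
; It has no other active logic: overlap and Tick are disabled, and the construction script only calls its parent.
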(event `self.ReceiveBeginPlay`
  (`parent.ReceiveBeginPlay`)
  (bind _asbp_game_state (cast `/Game/Variant_Strategy/Blueprints/BP_GameState` (`GameplayStatics.GetGameState`)))
  (set `/Game/Variant_Strategy/Blueprints/BP_GameState.Base` self _asbp_game_state))

(fn `UserConstructionScript`
  (`parent.UserConstructionScript`))